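; Character traversal component that manages travel state (free roam, ready to climb, climb, mantle, vault), climb style and climb direction.
; InitRef caches character references, including motion warping and camera, and attaches a spawned direction arrow actor above the mesh.
; Gameplay-tag setters act only on change and message the AnimInstance; travel state also switches capsule collision and movement mode.
; A helper picks between braced and free-hang values by climb style.
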(fn `ClimbStyleValue`
  (params (ClimbStyle :type "GameplayTag Structure") (Braced :type "Float (double-precision)") (FreeHang :type "Float (double-precision)"))
  (returns (Return :type "Float (double-precision)"))
  (`|SwitchGameplayTag` ClimbStyle
    (:`Traversal.ClimbStyle.BracedClimb`
      (return Braced))
    (:`Traversal.ClimbStyle.FreeHang`
      (return FreeHang))))

(fn `InitRef`
  (params (CharacterObjectRef :type "Character Object Reference") (MotionWarpingComponent :type "MotionWarpingComponent Object Reference") (CameraComponent :type "CameraComponent Object Reference"))
  (bind _character (`self.Character`))
  (bind _characterdirectionactor (`self.CharacterDirectionActor`))
  (bind _output_get (set `self.Character` CharacterObjectRef))
  (set `self.Character Movement` (`Character.CharacterMovement` _output_get))
  (bind _output_get_2 (set `self.Mesh` (`Character.Mesh` _output_get)))
  (set `self.Capsule Component` (`Character.CapsuleComponent` _output_get))
  (set `self.AnimInstatce` (`SkeletalMeshComponent.GetAnimInstance` _output_get_2))
  (set `self.Motion Warping Component` MotionWarpingComponent)
  (set `self.Camera Component` CameraComponent)
  (bind _returnvalue (`|SpawnActorFromClass` "/Game/TravelSystem/Actors/BP_CharakterDirectionArrow.BP_CharakterDirectionArrow_C" (`Actor.GetTransform` _character) "Undefined" "MultiplyWithRoot" _character null))
  (set `self.CharacterDirectionActor` _returnvalue)
  (`Actor.K2_AttachToComponent` _characterdirectionactor (`self.Mesh`) "None" "SnapToTarget" "SnapToTarget" "SnapToTarget" true)
  (`Actor.K2_SetActorRelativeLocation` _characterdirectionactor (0.0 0.0 195.0) false false))

(fn `SetClimbDirection`
  (params (NewClimbDirection :type "GameplayTag Structure"))
  (if (!= (`self.ClimbDirection`) NewClimbDirection)
    (bind _output_get (set `self.ClimbDirection` NewClimbDirection))
    (message `/Game/TravelSystem/Interface/I_Travel_APB.SetClimbDirection` (`self.AnimInstatce`) _output_get)))

(fn `SetClimbStyle`
  (params (NewClimbStyle :type "GameplayTag Structure"))
  (if (!= (`self.ClimbStyle`) NewClimbStyle)
    (bind _output_get (set `self.ClimbStyle` NewClimbStyle))
    (message `/Game/TravelSystem/Interface/I_Travel_APB.SetClimbStyle` (`self.AnimInstatce`) _output_get)))

(fn `SetTravelState`
  (params (NewTravelState :type "GameplayTag Structure"))
  (if (!= (`self.TravelState`) NewTravelState)
    (bind _output_get (set `self.TravelState` NewTravelState))
    (message `/Game/TravelSystem/Interface/I_Travel_APB.SetTravelState` (`self.AnimInstatce`) _output_get)
    (`|SwitchGameplayTag` _output_get
      (:`Traversal.State.FreeRoam`
        (`self.TravelStateSettings` "QueryAndPhysics" "MOVE_Walking"))
      (:`Traversal.State.ReadyToClimb`
        (`self.TravelStateSettings` "NoCollision" "MOVE_Flying"))
      (:`Traversal.State.Climb`
        (`self.TravelStateSettings` "NoCollision" "MOVE_Falling" true))
      (:`Traversal.State.Mantle`
        (`self.TravelStateSettings` "NoCollision" "MOVE_Flying"))
      (:`Traversal.State.Vault`
        (`self.TravelStateSettings` "NoCollision" "MOVE_Flying")))))

(fn `TravelStateSettings`
  (params (CollisionType :type "ECollisionEnabled Enum" :default "NoCollision") (NewMovementMode :type "EMovementMode Enum" :default "MOVE_None") (StopMovementImmediately :type Boolean))
  (bind _character_movement (`self.Character Movement`))
  (`PrimitiveComponent.SetCollisionEnabled` (`self.Capsule Component`) CollisionType)
  (`CharacterMovementComponent.SetMovementMode` _character_movement NewMovementMode 0)
  (if (`local.StopMovementImmediately`)
    (`MovementComponent.StopMovementImmediately` _character_movement)))